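; BP_Lift is a lift actor that moves vertically when the first-person character enters its trigger box.
; BeginPlay records the starting Z and adds LiftHeight to get the top height.
; Each box overlap flips a FlipFlop that alternately plays and reverses LiftTimeline, whose Height track lerps the actor's Z between the two heights while keeping X and Y.
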(event OnComponentBeginOverlap(Box)
  (params (OverlappedComponent :type Primitive%20Component%20Object%20Reference) (OtherActor :type Actor%20Object%20Reference) (OtherComp :type Primitive%20Component%20Object%20Reference) (OtherBodyIndex :type Integer) (bFromSweep :type Boolean) (SweepResult :type Hit%20Result%20Structure%20%28by%20ref%29))
  (Utilities|Casting|CastToFirstPersonCharacter OtherActor)
  (CallFunction|OnBoxTriggered))

(event Custom|OnBoxTriggered
  (bind _returnvalue (Transformation|GetActorLocation))
  (Utilities|FlowControl|FlipFlop
    (:A
      (bind _height (Timeline|LiftTimeline Play)
        (:Update
          (Transformation|SetActorLocation (Math|Vector|MakeVector (.x _returnvalue) (.y _returnvalue) (Math|Float|Lerp (Variables|Default|GetStartingHeight) (Variables|Default|GetEndingHeight) _height)) false false))))
    (:B
      (Timeline|LiftTimeline Reverse))))

(event EventBeginPlay
  (Variables|Default|SetStartingHeight (.z (Transformation|GetActorLocation)))
  (Variables|Default|SetEndingHeight (+ (Variables|Default|GetStartingHeight) (Variables|Default|GetLiftHeight))))

(event Collision|EventActorBeginOverlap
  (params (OtherActor :type Actor%20Object%20Reference)))

(event EventTick
  (params (DeltaSeconds :type Float%20%28single-precision%29)))

(fn ConstructionScript)